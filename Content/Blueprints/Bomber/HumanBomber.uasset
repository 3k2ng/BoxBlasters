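; Player-controlled bomber character that moves on input and drops bombs in the arena.
; On BeginPlay it runs the parent logic and has player controller 0 possess it, assuming only one human bomber exists.
; Move X and Move Y axis events share one AddMovementInput call.
; Space, if a bomb is available, spawns a NormalBomb on the current tile, registers it with the Arena, activates it and consumes a bomb.
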(event `self.ReceiveBeginPlay`
  ;[1 1 1] There should only be one Human Bomber, so we can just give it Player Controller 0
  (`parent.ReceiveBeginPlay`)
  (`Controller.Possess` (`GameplayStatics.GetPlayerController` 0) self))

(event `InputAxis|Move X`
  (params (AxisValue :type "Float (single-precision)"))
  (`self.AddMovementInput` (`KismetMathLibrary.MakeVector` AxisValue (stale `InputAxis|Move Y` AxisValue)) :!label _label))

(event `InputAxis|Move Y`
  (params (AxisValue :type "Float (single-precision)"))
  (goto _label))

(event `Key|SpaceBar`
  (params (Key :type "Key Structure"))
  (:`Pressed`
    (if (`self.IsBombAvailable`)
      (bind _returnvalue (`|SpawnActorFromClass` "/Game/Blueprints/Bomb/NormalBomb.NormalBomb_C" (`KismetMathLibrary.MakeTransform` (`CommonUtils.GetTileLocation` (`self.GetCurrentTile`))) "Undefined" "OverrideRootScale" null null))
      (`Bomb.SetBomber` _returnvalue self)
      (`Arena.PlaceBomb` (`self.Arena`) "Normal" (`Bomb.GetCurrentTile` _returnvalue) (`self.Power`))
      (`Bomb.Activate` _returnvalue)
      (`self.ConsumeBomb`))))

(fn `UserConstructionScript`)