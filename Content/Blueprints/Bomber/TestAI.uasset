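; Test AI bomber that exercises bomb-aware A* pathfinding from itself toward a fixed goal tile.
; On begin play, a looping timer requests the path using the bomber's power, a bomb cost and a weight, then logs each tile's world location.
; A separate one-shot timer applies a single power-up shortly after start.
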(event `self.ReceiveBeginPlay`
  (`parent.ReceiveBeginPlay`)
  (`KismetSystemLibrary.K2_SetTimerDelegate` (delegate `AiLoop`) 2.0 true)
  (`KismetSystemLibrary.K2_SetTimerDelegate` (delegate `Buff`) 1.0))

(event `AiLoop`
  (for _array_element (`RobotUtils.GetBombAStar` self (make `Tile` 14 12) (`self.Power`) 10 20)
    (`VisualLoggerKismetLibrary.LogLocation` null (`CommonUtils.GetTileLocation` _array_element) "" (struct :`B` 1.0 :`A` 1.0) 100.0)))

(event `Buff`
  (`self.PowerUp`))

(fn `UserConstructionScript`
  (`parent.UserConstructionScript`))