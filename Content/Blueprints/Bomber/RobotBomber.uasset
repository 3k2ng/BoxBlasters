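; Base AI bomber that runs a queue of Move, Wait, Strike, Bomb and Special tasks.
; Each Tick calls a BeforeQueueProcess hook, steers any deployed air strike, then processes the front task or calls OnQueueEmpty; both hooks are empty here.
; Moves follow A* with safe and danger tile costs, while waits hold until the target is safely reachable.
; Pickups, failed actions, missing paths and unsafe waits clear the queue.
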(event `self.ReceiveBeginPlay`
  ;[1 1 1] Create an AI Controller at BeginPlay, also initialize Destination at current Tile
  (`parent.ReceiveBeginPlay`)
  (`self.SpawnDefaultController`))

(event `self.OnPickUp`
  (`self.Halt`))

(event `self.ReceiveTick`
  (params (DeltaSeconds :type "Float (single-precision)"))
  (bind (_tasktype _target) (break `RobotTask` (`self.QueueTop`)))
  (`parent.ReceiveTick` DeltaSeconds)
  (`self.BeforeQueueProcess`)
  (`self.StrikeMove`
    (:`Out`
      (if (`self.QueueEmpty`)
        (`self.OnQueueEmpty`)
        (else
          (switch `ERobotTaskType` _tasktype
            (:`Move`
              (`self.ProcessMoveTask` _target))
            (:`Wait`
              (`self.ProcessWaitTask` _target))
            (:`Strike`
              (set `self.StrikeDestination` _target)
              (`self.QueuePop` :!label _label))
            (:`Bomb`
              (bind _returnvalue (`self.PlaceBomb`))
              (if _returnvalue
                (goto _label)
                (else
                  (`self.Halt` :!label _label_2))))
            (:`Special`
              (bind _returnvalue_2 (`self.ActivateSpecial`))
              (if _returnvalue_2
                (goto _label)
                (else
                  (goto _label_2))))))))))

(event `BeforeQueueProcess`)

(event `OnQueueEmpty`)

(fn `DoBomb`
  (`KismetArrayLibrary.Array_Add` (`self.TaskQueue`) (make `RobotTask` "Bomb")))

(fn `DoSpecial`
  (`KismetArrayLibrary.Array_Add` (`self.TaskQueue`) (make `RobotTask` "Special")))

(fn `Halt`
  (`KismetArrayLibrary.Array_Clear` (`self.TaskQueue`)))

(fn `IsDestinationReach`
  (params (Destination :type "Tile Structure"))
  (returns (ReturnValue :type Boolean))
  (return (<= (`KismetMathLibrary.Vector_Distance` (`CommonUtils.GetTileLocation` Destination) (`self.K2_GetActorLocation`)) 20.0)))

(fn `IsStrikeDestinationReach`
  (returns (ReturnValue :type Boolean))
  (if (`KismetSystemLibrary.IsValid` (`self.DeployedAirStrike`))
    (return (<= (`KismetMathLibrary.Vector_Distance` (`CommonUtils.GetTileLocation` (`self.StrikeDestination`)) (`self.K2_GetActorLocation` (`self.DeployedAirStrike`))) 20.0))
    (else
      (return true))))

(fn `MoveTo`
  (params (Destination :type "Tile Structure"))
  (`KismetArrayLibrary.Array_Add` (`self.TaskQueue`) (make `RobotTask` "Move" Destination)))

(fn `QueueEmpty`
  (returns (QueueEmpty :type Boolean))
  (return (<= (`KismetArrayLibrary.Array_Length` (`self.TaskQueue`)) 0)))

(fn `QueuePop`
  (`KismetArrayLibrary.Array_Remove` (`self.TaskQueue`)))

(fn `QueueTop`
  (returns (Top :type "RobotTask Structure"))
  (return (`|GetArrayItem` (`self.TaskQueue`))))

(fn `ReachablePickUps`
  (params (FindUpgrade :type Boolean) (FindSpecial :type Boolean) (FindRed :type Boolean) (FindGreen :type Boolean) (FindBlue :type Boolean))
  (returns (Results :type "Array of Tile Structure"))
  (return (`RobotUtils.FilterReachable` self (`PlanningUtils.GetPickUps` self FindUpgrade FindSpecial FindRed FindGreen FindBlue) true)))

(fn `StrikeTo`
  (params (Target :type "Tile Structure"))
  (`KismetArrayLibrary.Array_Add` (`self.TaskQueue`) (make `RobotTask` "Strike" Target)))

(fn `UserConstructionScript`)

(fn `WaitFor`
  (params (Target :type "Tile Structure"))
  (`KismetArrayLibrary.Array_Add` (`self.TaskQueue`) (make `RobotTask` "Wait" Target)))