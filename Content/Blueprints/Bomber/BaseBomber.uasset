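; BaseBomber is a base Blueprint for a bomber character that animates its Paper2D sprite from movement input.
; Each Tick calls the parent Tick, then switches the flipbook between walk and idle based on the last movement input vector.
; While walking, it mirrors the sprite by negating its X scale for leftward input, and idle restores the unflipped scale.
; The OnPickUp event is an empty stub.
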(event `self.ReceiveTick`
  (params (DeltaSeconds :type "Float (single-precision)"))
  (bind _returnvalue_x (`KismetMathLibrary.BreakVector` (`self.GetLastMovementInputVector`)))
  (bind _paperflipbook (`self.PaperFlipbook`))
  (bind _paperflipbook_2 (`self.PaperFlipbook`))
  (`parent.ReceiveTick` DeltaSeconds)
  (if (> (`KismetMathLibrary.VSize` (`self.GetLastMovementInputVector`)) 0.1)
    (`PaperFlipbookComponent.SetFlipbook` _paperflipbook "/Game/Sprites/Bomber/FB_Bomber_Walk.FB_Bomber_Walk")
    (if (< _returnvalue_x 0.0)
      (`SceneComponent.SetRelativeScale3D` _paperflipbook_2 (-0.6 0.6 0.6))
      (else
        (`SceneComponent.SetRelativeScale3D` _paperflipbook_2 (0.6 0.6 0.6))))
    (else
      (`PaperFlipbookComponent.SetFlipbook` _paperflipbook "/Game/Sprites/Bomber/FB_Bomber_Idle.FB_Bomber_Idle")
      (`SceneComponent.SetRelativeScale3D` (`self.PaperFlipbook`) (0.6 0.6 0.6)))))

(event `OnPickUp`)

(fn `UserConstructionScript`)