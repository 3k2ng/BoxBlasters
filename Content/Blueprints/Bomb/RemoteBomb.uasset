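; RemoteBomb is a bomb variant that explodes when its Detonate event is called, telling the Arena to detonate the bomb on its current tile and then destroying itself.
; Its collision box switches to BlockAll once the Bomber stops overlapping it.
; Each tick runs the parent logic, then destroys the actor without calling Detonate if the CheckBombMap check fails.
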(event `self.Activate`
  (`parent.Activate`))

(event `self.Detonate`
  (`Arena.DetonateBomb` (`self.Arena`) (`self.GetCurrentTile`))
  (`self.K2_DestroyActor`))

(event `self.ReceiveActorEndOverlap`
  (params (OtherActor :type "Actor Object Reference"))
  (if (== OtherActor (`self.Bomber`))
    (`PrimitiveComponent.SetCollisionProfileName` (`self.Box`) "BlockAll" true)))

(event `self.ReceiveTick`
  (params (DeltaSeconds :type "Float (single-precision)"))
  (`parent.ReceiveTick` DeltaSeconds)
  (if (not (`self.CheckBombMap`))
    (`self.K2_DestroyActor`)))

(fn `UserConstructionScript`)