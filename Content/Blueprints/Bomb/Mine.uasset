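; Mine is a bomb actor that arms after its Bomber steps off it, then detonates when an actor next stops overlapping it.
; Detonation passes the mine's current tile to the Arena's DetonateBomb, then destroys the actor.
; Each tick runs the parent logic and removes the mine without detonating if CheckBombMap fails.
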(event `self.Detonate`
  (`Arena.DetonateBomb` (`self.Arena`) (`self.GetCurrentTile`))
  (`self.K2_DestroyActor`))

(event `self.ReceiveActorEndOverlap`
  (params (OtherActor :type "Actor Object Reference"))
  (if (`self.IsActive`)
    (`self.Detonate`)
    (elif (== OtherActor (`self.Bomber`))
      (set `self.IsActive` true))))

(event `self.ReceiveTick`
  (params (DeltaSeconds :type "Float (single-precision)"))
  (`parent.ReceiveTick` DeltaSeconds)
  (if (not (`self.CheckBombMap`))
    (`self.K2_DestroyActor`)))

(fn `UserConstructionScript`)