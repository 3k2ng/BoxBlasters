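; NormalBomb is a timed bomb that a Bomber places on an Arena tile.
; Activation starts a fixed, non-looping timer, after which the bomb tells the Arena to detonate at its current tile, replenishes the Bomber's bomb and destroys itself.
; Its Box switches to the BlockAll collision profile once the owning Bomber stops overlapping it, so the bomb becomes solid only after its placer steps off.
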(event `self.Activate`
  (`KismetSystemLibrary.K2_SetTimerDelegate` (delegate `self.Detonate`) 2.0))

(event `self.Detonate`
  (`Arena.DetonateBomb` (`self.Arena`) (`self.GetCurrentTile`))
  (`Bomber.ReplenishBomb` (`self.Bomber`))
  (`self.K2_DestroyActor`))

(event `self.ReceiveActorEndOverlap`
  (params (OtherActor :type "Actor Object Reference"))
  (if (== OtherActor (`self.Bomber`))
    (`PrimitiveComponent.SetCollisionProfileName` (`self.Box`) "BlockAll" true)))

(fn `UserConstructionScript`)