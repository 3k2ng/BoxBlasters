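; BasePickUp is a collectible that grants a bomber either a stat upgrade or a special item.
; Each tick it checks for overlapping ArmedBomber actors and acts on the first, cast to BaseBomber.
; Type picks the category and Color the effect: power, speed or bomb upgrades, or a Remote, Air or Mine special via GetSpecial.
; It notifies the bomber and destroys itself, but a special only if equipping succeeds.
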(event `self.ReceiveTick`
  (params (DeltaSeconds :type "Float (single-precision)"))
  (bind _overlappingactors (`self.GetOverlappingActors` "/Script/BoxBlasters.ArmedBomber"))
  (`parent.ReceiveTick` DeltaSeconds)
  (if (> (`KismetArrayLibrary.Array_Length` _overlappingactors) 0)
    (bind _asbase_bomber (cast `/Game/Blueprints/Bomber/BaseBomber` (`|GetArrayItem` _overlappingactors)))
    (switch `EPickUpType` (`self.Type`)
      (:`Upgrade`
        (switch `EPickUpColor` (`self.Color`)
          (:`Red`
            (`Bomber.PowerUp` _asbase_bomber))
          (:`Green`
            (`Bomber.SpeedUp` _asbase_bomber))
          (:`Blue`
            (`Bomber.BombUp` _asbase_bomber)))
        (`/Game/Blueprints/Bomber/BaseBomber.OnPickUp` _asbase_bomber :!label _label)
        (`self.K2_DestroyActor`))
      (:`Special`
        (bind _returnvalue (`ArmedBomber.EquipSpecial` _asbase_bomber (`self.GetSpecial`)))
        (if _returnvalue
          (goto _label))))))

(fn `GetSpecial`
  (returns (Special :type "ESpecialType Enum"))
  (switch `EPickUpColor` (`self.Color`)
    (:`Red`
      (return "Remote"))
    (:`Green`
      (return "Air"))
    (:`Blue`
      (return "Mine"))))

(fn `UserConstructionScript`)